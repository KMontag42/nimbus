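; NIMBUS_DamageSource is a short-lived damage volume actor that destroys itself after its TTL lifespan.
; On overlap with any actor other than its owner, it applies its configured damage amount and damage type, naming itself as the causer.
; GetKnockbackVector scales the Knockback value by a magnitude along an XZ direction with Y zeroed, but this file never calls it.
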(event EventBeginPlay
  (Actor|SetLifeSpan (Variables|Default|GetTTL)))

(event Collision|EventActorBeginOverlap
  (params (OtherActor :type Actor%20Object%20Reference))
  (if (!= OtherActor (Components|GetOwner))
    (Game|Damage|ApplyDamage OtherActor (Variables|Default|GetDamageAmount) 0 self (Variables|Default|GetDamageType))))

(fn ConstructionScript)

(fn GetKnockbackVector
  (params (Magnitude :type Float%20%28single-precision%29) (XDirection :type Vector) (ZDirection :type Vector))
  (return (* (* (Variables|Default|GetKnockback) (Math|Vector|MakeVector (.X (Math|Vector|BreakVector XDirection)) 0.0 (.Z (Math|Vector|BreakVector ZDirection)))) Magnitude)))