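; Player state machine for NIMBUS_Actor that drives Paper2D flipbooks for movement, attack, hurt and death states.
; Per-state Begin/Update/Finish functions swap flipbooks and use velocity, jump readiness or timers to change or finish states.
; One-shot states finish after a delay equal to their flipbook's duration.
; Attacks, smashes, hurt and death lock input; Attack spawns a damage source at AttackArrow, and Death triggers respawn.
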(event EventEventonUpdateState
  (params (CurrentState :type Byte :default 0) (StateName :type Name) (StateTimer :type Float%20%28single-precision%29))
  (switch name StateName
    (:StartRun
      _)
    (:Land
      _)
    (:Stop
      _)
    (:Attack
      _)
    (:DownSmash
      _)
    (:UpSmash
      _))
  (bind _returnvalue (CallFunction|GetOwnerFlipbookDuration))
  (Utilities|FlowControl|Delay _returnvalue)
  (Class|StateMachineComponent|FinishState))

(fn OnBeginIdle
  (bind _actor (CallFunction|GetOwnerCharacter))
  (Sprite|SetFlipbook (Variables|/Game/Actors/NIMBUS_Actor.NIMBUS_Actor_C|GetPaperFlipbook _actor) "/Game/Resources/alucard/idle/1_Sprite1.1_Sprite1"))

(fn OnUpdateIdle)

(fn OnExitIdle)

(fn OnFinishIdle)

(fn OnBeginRun
  (bind _actor (CallFunction|GetOwnerCharacter))
  (Variables|/Game/Actors/NIMBUS_Actor.NIMBUS_Actor_C|SetVelocityMultiplier _actor 1.0)
  (Sprite|SetFlipbook (Variables|/Game/Actors/NIMBUS_Actor.NIMBUS_Actor_C|GetPaperFlipbook _actor) "/Game/Resources/alucard/walking/Run.Run"))

(fn OnUpdateRun
  (bind _actor (CallFunction|GetOwnerCharacter))
  (if (== (.X (Math|Vector|BreakVector (Transformation|GetVelocity _actor))) 0.0)
    (Class|StateMachineComponent|FinishState)))

(fn OnExitRun)

(fn OnFinishRun)

(fn OnBeginStartRun
  (CallFunction|SetOwnerFlipbook "/Game/Resources/alucard/runstart/StartRun.StartRun"))

(fn OnUpdateStartRun
  (CallFunction|ManualJumpTransition)
  (bind _actor (CallFunction|GetOwnerCharacter))
  (if (== (.X (Math|Vector|BreakVector (Transformation|GetVelocity _actor))) 0.0)
    (Class|StateMachineComponent|SetState "Stop")))

(fn OnExitStartRun)

(fn OnFinishStartRun)

(fn GetOwnerCharacter
  (bind _asnimbus_actor (Utilities|Casting|CastToNIMBUS_Actor (Components|GetOwner)))
  (return _asnimbus_actor))

(fn OnBeginJump
  (bind _actor (CallFunction|GetOwnerCharacter))
  (Sprite|SetFlipbook (Variables|/Game/Actors/NIMBUS_Actor.NIMBUS_Actor_C|GetPaperFlipbook _actor) "/Game/Resources/alucard/jump/Jump.Jump"))

(fn OnUpdateJump
  (bind _returnvalue (CallFunction|GetOwnerVelocity))
  (if (<= (.Z (Math|Vector|BreakVector _returnvalue)) 0.0)
    (Class|StateMachineComponent|FinishState)
    (elif (!= (.X (Math|Vector|BreakVector _returnvalue)) 0.0)
      (CallFunction|SetOwnerFlipbook "/Game/Resources/alucard/jumpmove/JumpMove.JumpMove"))))

(fn OnExitJump)

(fn OnFinishJump)

(fn OnBeginFall
  (bind _actor (CallFunction|GetOwnerCharacter))
  (Sprite|SetFlipbook (Variables|/Game/Actors/NIMBUS_Actor.NIMBUS_Actor_C|GetPaperFlipbook _actor) "/Game/Resources/alucard/fall/Fall.Fall"))

(fn OnUpdateFall
  (bind _actor (CallFunction|GetOwnerCharacter))
  (if (Character|CanJump _actor)
    (Class|StateMachineComponent|FinishState)))

(fn OnExitFall)

(fn OnFinishFall)

(fn OnBeginStop
  (CallFunction|SetOwnerFlipbook "/Game/Resources/alucard/stop/Stop.Stop"))

(fn OnUpdateStop
  (CallFunction|ManualRunTransition))

(fn OnExitStop)

(fn OnFinishStop)

(fn OnBeginTurnAround)

(fn OnUpdateTurnAround)

(fn OnExitTurnAround)

(fn OnFinishTurnAround)

(fn OnBeginLand
  (CallFunction|SetOwnerFlipbook "/Game/Resources/alucard/land/Land.Land"))

(fn OnUpdateLand
  (CallFunction|ManualRunTransition))

(fn OnExitLand)

(fn OnFinishLand)

(fn OnBeginAttack
  (CallFunction|SetOwnerCanMove false)
  (CallFunction|SetOwnerFlipbook "/Game/Resources/alucard/attack/Attack.Attack")
  (bind _actor (CallFunction|GetOwnerCharacter))
  (bind _returnvalue (Game|SpawnActorfromClass "/Game/Blueprints/DamageSources/NIMBUS_Player_Attack_DamageSource.NIMBUS_Player_Attack_DamageSource_C" (Transformation|GetWorldTransform (Variables|/Game/Actors/NIMBUS_Actor.NIMBUS_Actor_C|GetAttackArrow _actor)) "Undefined" _actor 0))
  (Variables|/Game/Blueprints/NIMBUS_DamageSource.NIMBUS_DamageSource_C|SetParent _returnvalue _actor))

(fn OnUpdateAttack)

(fn OnExitAttack)

(fn OnFinishAttack
  (CallFunction|SetOwnerCanMove true))

(fn OnBeginUpSmash
  (CallFunction|SetOwnerCanMove false)
  (CallFunction|SetOwnerFlipbook "/Game/Resources/alucard/upsmash/UpSmash.UpSmash"))

(fn OnUpdateUpSmash)

(fn OnExitUpSmash)

(fn OnFinishUpSmash
  (CallFunction|SetOwnerCanMove true))

(fn OnBeginDownSmash
  (CallFunction|SetOwnerCanMove false)
  (CallFunction|SetOwnerFlipbook "/Game/Resources/alucard/downsmash/Downsmash.Downsmash"))

(fn OnUpdateDownSmash)

(fn OnExitDownSmash)

(fn OnFinishDownSmash
  (CallFunction|SetOwnerCanMove true))

(fn OnBeginHurt
  (CallFunction|SetOwnerFlipbook "/Game/Resources/alucard/hurt/Hurt.Hurt")
  (CallFunction|SetOwnerCanMove false))

(fn OnUpdateHurt
  (if (>= (Class|StateMachineComponent|GetTime) 1.0)
    (Class|StateMachineComponent|FinishState)))

(fn OnExitHurt)

(fn OnFinishHurt
  (CallFunction|SetOwnerCanMove true))

(fn SetOwnerFlipbook
  (params (NewFlipbook :type Paper%20Flipbook%20Object%20Reference))
  (bind _actor (CallFunction|GetOwnerCharacter))
  (Sprite|SetFlipbook (Variables|/Game/Actors/NIMBUS_Actor.NIMBUS_Actor_C|GetPaperFlipbook _actor) NewFlipbook))

(fn GetOwnerFlipbook
  (bind _actor (CallFunction|GetOwnerCharacter))
  (return (Class|PaperFlipbookComponent|GetFlipbook (Variables|/Game/Actors/NIMBUS_Actor.NIMBUS_Actor_C|GetPaperFlipbook _actor))))

(fn GetOwnerFlipbookDuration
  (bind _returnvalue (CallFunction|GetOwnerFlipbook))
  (return (Class|PaperFlipbook|GetTotalDuration _returnvalue)))

(fn GetOwnerVelocity
  (bind _actor (CallFunction|GetOwnerCharacter))
  (return (Transformation|GetVelocity _actor)))

(fn SetOwnerCanMove
  (params (Condition :type Boolean))
  (bind _actor (CallFunction|GetOwnerCharacter))
  (if Condition
    (Variables|/Game/Actors/NIMBUS_Actor.NIMBUS_Actor_C|SetCanTakeInput _actor true)
    (else
      (Variables|/Game/Actors/NIMBUS_Actor.NIMBUS_Actor_C|SetCanTakeInput _actor false))))

(fn OnBeginDeath
  (CallFunction|SetOwnerFlipbook "/Game/Resources/alucard/death/Death.Death")
  (CallFunction|SetOwnerCanMove false))

(fn OnUpdateDeath
  (if (>= (Class|StateMachineComponent|GetTime) 1.0)
    (bind _actor (CallFunction|GetOwnerCharacter))
    (Default|Respawn _actor)))

(fn OnExitDeath
  (CallFunction|SetOwnerCanMove true))

(fn OnFinishDeath)

(fn ManualRunTransition
  (bind _returnvalue (CallFunction|GetOwnerVelocity))
  (if (!= (.X (Math|Vector|BreakVector _returnvalue)) 0.0)
    (Class|StateMachineComponent|SetState "Run")))

(fn ManualJumpTransition
  (bind _returnvalue (CallFunction|GetOwnerVelocity))
  (if (> (.Z (Math|Vector|BreakVector _returnvalue)) 0.0)
    (Class|StateMachineComponent|SetState "Jump")))