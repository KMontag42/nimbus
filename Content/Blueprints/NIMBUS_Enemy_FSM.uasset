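; Finite state machine logic for a NIMBUS enemy, with states to search for the player, wait, approach and attack.
; Search caches the first valid player actor as the target.
; Approach feeds only the X component of the direction to that target into the owner's move input, finishing within attack range.
; Attack repeats attack input until it returns true; Waiting is empty, and transitions are not defined here.
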(fn OnBeginSearchforPlayer
  (bind _outactors (Actor|GetAllActorsOfClass "/Game/Actors/NIMBUS_Player_Actor.NIMBUS_Player_Actor_C"))
  (bind _array_element (Utilities|Array|ForEachLoopwithBreak _outactors :!label _label)
    (:LoopBody
      (Utilities|IsValid _array_element
        (:Is%20Valid
          (Variables|Default|SetTargetActor _array_element)
          (goto _label Break))))
    (:Completed
      (Class|StateMachineComponent|FinishState))))

(fn OnUpdateSearchforPlayer)

(fn OnExitSearchforPlayer)

(fn OnFinishSearchforPlayer)

(fn OnBeginWaiting)

(fn OnUpdateWaiting)

(fn OnExitWaiting)

(fn OnFinishWaiting)

(fn OnBeginApproach)

(fn OnUpdateApproach
  (bind _targetactor (Variables|Default|GetTargetActor))
  (bind _actor (CallFunction|GetOwnerActor self))
  (Default|OnMoveInput _actor (.X (Math|Vector|BreakVector (Math|Vector|GetUnitDirection(Vector) (Transformation|GetActorLocation _actor) (Transformation|GetActorLocation _targetactor)))))
  (if (< (Transformation|GetDistanceTo _actor _targetactor) (Variables|Default|GetAttackRange))
    (Class|StateMachineComponent|FinishState)))

(fn OnExitApproach)

(fn OnFinishApproach)

(fn OnBeginAttack)

(fn OnUpdateAttack
  (bind _actor (CallFunction|GetOwnerActor self))
  (bind _didattack (Default|OnAttackInput _actor true))
  (if _didattack
    (Class|StateMachineComponent|FinishState)))

(fn OnExitAttack)

(fn OnFinishAttack)